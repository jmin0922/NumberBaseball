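; Game mode for a chat-based number-guessing game that scores players' guesses as strikes, balls or outs against a random number generated at BeginPlay.
; PostLogin registers each BP_ChatPC in a map with zeroed S/B counts and a numbered player name.
; CalculateSBO passes a guess and that player's counts to GetSBO, stores the updated counts, then broadcasts the name-prefixed result to every chat controller through FromServer.
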(event `self.ReceiveBeginPlay`
  (bind _returnvalue (`NBFunctionLibrary.GenerateRandomNum`))
  (set `self.RandomNum` _returnvalue))

(event `CalculateSBO`
  (params (ChatPC :type "/Game/Chat/BP_ChatPC Object Reference") (MyNumber :type String))
  (bind _value (`BlueprintMapLibrary.Map_Find` (`self.AllPCs`) (`self.Chat PC`)))
  (`|ExecutionSequence`
    (:`then_0`
      (set `self.Chat PC` ChatPC)
      (set `self.My Number` MyNumber))
    (:`then_1`
      (if true
        (bind (_outs _outb _outmsg) (`NBFunctionLibrary.GetSBO` (`self.My Number`) (`self.RandomNum`) (break `/Game/Chat/ST_PlayerInfo` _value) (`.B_7_1D0A3C3C4E1199D9994E6E9BA75687E7` (break `/Game/Chat/ST_PlayerInfo` _value))))
        (`BlueprintMapLibrary.Map_Add` (`self.AllPCs`) (`self.Chat PC`) (make `/Game/Chat/ST_PlayerInfo` _outs _outb (`.Name_8_2163865F4936EFE241E96098E89C5EA1` (break `/Game/Chat/ST_PlayerInfo` (`BlueprintMapLibrary.Map_Find` (`self.AllPCs`) (`self.Chat PC`))))))
        (`self.BroadCast` _outmsg)))))

(event `self.K2_PostLogin`
  (params (NewPlayer :type "PlayerController Object Reference"))
  (bind _asbp_chat_pc (cast `/Game/Chat/BP_ChatPC` NewPlayer))
  (`BlueprintMapLibrary.Map_Add` (`self.AllPCs`) _asbp_chat_pc (make `/Game/Chat/ST_PlayerInfo` 0 0 (`KismetTextLibrary.Conv_TextToString` (`|FormatText` "Player{0}" (`BlueprintMapLibrary.Map_Length` (`self.AllPCs`)))))))

(event `BroadCast`
  (params (Message :type String))
  (bind _outactors (`GameplayStatics.GetAllActorsOfClass` "/Game/Chat/BP_ChatPC.BP_ChatPC_C"))
  (for _array_element _outactors
    (`/Game/Chat/BP_ChatPC.FromServer` _array_element (`KismetTextLibrary.Conv_TextToString` (`|FormatText` "{0}:{1}" (`.Name_8_2163865F4936EFE241E96098E89C5EA1` (break `/Game/Chat/ST_PlayerInfo` (`BlueprintMapLibrary.Map_Find` (`self.AllPCs`) (`self.Chat PC`)))) Message)))))

(fn `UserConstructionScript`)