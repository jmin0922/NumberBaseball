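; Player controller for a chat-driven game in which the player's typed message is submitted as a number for the game mode's SBO calculation.
; On BeginPlay, the local controller creates WBP_Chat, shows the cursor and binds the widget's chat event.
; Messages go through ToServer to BP_ChatGameMode.CalculateSBO, though the MyPC argument is left unset.
; FromServer passes incoming messages back to the widget for display.
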(event `self.ReceiveBeginPlay`
  (if (`self.IsLocalPlayerController`)
    (bind _returnvalue (`|CreateWidget` "/Game/Chat/WBP_Chat.WBP_Chat_C"))
    (`UserWidget.AddToViewport` _returnvalue 0)
    (set `self.bShowMouseCursor` true)
    (add `/Game/Chat/WBP_Chat.ChatED` _returnvalue (delegate `FromWideget`))
    (`NBFunctionLibrary.MyPrintString` "Hello")))

(event `FromWideget`
  (params (ChatMessage :type String))
  (`self.ToServer` ChatMessage))

(event `FromServer`
  (params (ChatMessagre :type String))
  (`/Game/Chat/WBP_Chat.TOUI` (stale `self.ReceiveBeginPlay` _returnvalue) ChatMessagre))

(event `ToServer`
  (params (ChatMessage :type String) (`My PC` :type "/Game/Chat/BP_ChatPC Object Reference"))
  (bind _asbp_chat_game_mode (cast `/Game/Chat/BP_ChatGameMode` (`GameplayStatics.GetGameMode`)))
  (`/Game/Chat/BP_ChatGameMode.CalculateSBO` _asbp_chat_game_mode `My PC` ChatMessage))

(fn `UserConstructionScript`)